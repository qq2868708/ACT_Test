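; PickableItem_BP is a pickup that grants the Hades_BP player one SkillCount in its Inventory_BP component.
; A timeline (旋转) started on BeginPlay drives its yaw spin.
; Each Tick, while the player is within a set radius, it homes in with growing Speed, applied per frame without delta-time scaling.
; At very close range it increments the count and destroys itself.
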(event EventBeginPlay
  (bind _newtrack_0 (Timeline|旋转 Play)
    (:Update
      (Transformation|SetActorRotation (Math|Rotator|MakeRotator 0.0 0.0 (* 360 _newtrack_0))))))

(event EventTick
  (params (DeltaSeconds :type Float%20%28single-precision%29))
  (bind _returnvalue (Game|GetPlayerCharacter 0))
  (bind _returnvalue_2 (Transformation|GetActorLocation))
  (bind _returnvalue_3 (Transformation|GetActorLocation _returnvalue))
  (bind _returnvalue_4 (- _returnvalue_3 _returnvalue_2))
  (if (<= (Math|Vector|VectorLength _returnvalue_4) 3e+02)
    (bind _output_get (Variables|Default|SetSpeed (+ (Variables|Default|GetSpeed) (* 10 DeltaSeconds))))
    (Transformation|SetActorLocation (+ _returnvalue_2 (* (Math|Vector|Normalize _returnvalue_4) _output_get)) false false)
    (if (<= (Math|Vector|VectorLength (- (Transformation|GetActorLocation) _returnvalue_3)) 1e+01)
      (bind _ashades_bp (Utilities|Casting|CastToHades_BP (Game|GetPlayerCharacter 0)))
      (Variables|/Game/Hades/Character/Inventory_BP.Inventory_BP_C|SetSkillCount (Actor|GetComponentbyClass _ashades_bp "/Game/Hades/Character/Inventory_BP.Inventory_BP_C") (+ (Variables|/Game/Hades/Character/Inventory_BP.Inventory_BP_C|GetSkillCount (Actor|GetComponentbyClass _ashades_bp "/Game/Hades/Character/Inventory_BP.Inventory_BP_C")) 1))
      (Actor|DestroyActor))))

(fn ConstructionScript)