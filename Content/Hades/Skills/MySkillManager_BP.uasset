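; MySkillManager_BP is a skill manager that registers a fixed set of hit skills when play begins.
; BeginPlay calls AddSkill for each of the Hit1 to Hit4 and Hit5_Dash Blueprints, then adds each returned skill uniquely to SkillArray.
; It contains only this setup, with no activation logic and an empty, disabled Tick.
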(event EventBeginPlay
  (bind _returnvalue (Class|SkillManager|AddSkill "/Game/Hades/Skills/Hit1_BP.Hit1_BP_C"))
  (Utilities|Array|AddUnique (Variables|Default|GetskillArray) _returnvalue)
  (bind _returnvalue_2 (Class|SkillManager|AddSkill "/Game/Hades/Skills/Hit2_BP.Hit2_BP_C"))
  (Utilities|Array|AddUnique (Variables|Default|GetskillArray) _returnvalue_2)
  (bind _returnvalue_3 (Class|SkillManager|AddSkill "/Game/Hades/Skills/Hit3_BP.Hit3_BP_C"))
  (Utilities|Array|AddUnique (Variables|Default|GetskillArray) _returnvalue_3)
  (bind _returnvalue_4 (Class|SkillManager|AddSkill "/Game/Hades/Skills/Hit4_BP.Hit4_BP_C"))
  (Utilities|Array|AddUnique (Variables|Default|GetskillArray) _returnvalue_4)
  (bind _returnvalue_5 (Class|SkillManager|AddSkill "/Game/Hades/Skills/Hit5_Dash_BP.Hit5_Dash_BP_C"))
  (Utilities|Array|AddUnique (Variables|Default|GetskillArray) _returnvalue_5))

(event EventTick
  (params (DeltaSeconds :type Float%20%28single-precision%29)))