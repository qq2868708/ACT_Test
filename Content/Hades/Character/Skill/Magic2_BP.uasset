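; Homing magic skill projectile that sweeps forward, seeks a nearby pawn other than the player and turns toward it in yaw only.
; On hit, a sphere trace damages living BaseEnemy_BP pawns, then calls SetCount on the one nearest world origin (SelectMinDistance receives a zero vector).
; It spawns a PickableItem_BP when it exceeds its travel distance or its impact finds no pawns.
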(event Collision|EventHit
  (params (MyComp :type Primitive%20Component%20Object%20Reference) (Other :type Actor%20Object%20Reference) (OtherComp :type Primitive%20Component%20Object%20Reference) (bSelfMoved :type Boolean) (HitLocation :type Vector :default "0, 0, 0") (HitNormal :type Vector :default "0, 0, 0") (NormalImpulse :type Vector :default "0, 0, 0") (Hit :type Hit%20Result%20Structure%20%28by%20ref%29))
  (bind _returnvalue (Transformation|GetActorLocation))
  (bind _array (Variables|Default|GetArray))
  (bind _array_2 (Variables|Default|GetArray))
  ;[1 1 1] Comment
  (if (not (== Other (Variables|Default|GetOwnerActor)))
    (Variables|Default|SetSelfPos _returnvalue)
    (bind _outhits (Collision|MultiSphereTraceForObjects _returnvalue _returnvalue 1e+02 (Utilities|Array|MakeArray "ObjectTypeQuery3") false 0 "ForDuration" true "(R=1.000000,G=0.000000,B=0.000000,A=1.000000)" "(R=0.000000,G=1.000000,B=0.000000,A=1.000000)" 2.0))
    (if (<= (Utilities|Array|Length _outhits) 0)
      (bind _returnvalue_2 (Game|SpawnActorfromClass "/Game/Hades/Items/PickableItem_BP.PickableItem_BP_C" (Math|Transform|MakeTransform (Transformation|GetActorLocation) "0, 0, 0" "1,1,1") "Undefined" 0 0 :!label _label))
      (Transformation|SetMobility _returnvalue_2 "Movable")
      (Actor|DestroyActor)
      (else
        (for _array_element _outhits
          (Utilities|Array|AddUnique _array_2 (.hitactor _array_element)))
        (if (<= (Utilities|Array|Length _array_2) 0)
          (goto _label)
          (else
            (for _array_element_2 _array
              (bind _asbase_enemy_bp (Utilities|Casting|CastToBaseEnemy_BP _array_element_2))
              (if (not (Variables|/Game/Hades/AI/BaseAICharacter/BaseEnemy_BP.BaseEnemy_BP_C|GetDead _asbase_enemy_bp))
                (Default|SetCauserSource _asbase_enemy_bp (Variables|Default|GetSelfPos))
                (Game|Damage|ApplyDamage _array_element_2 45.0 0 0 "/Game/Hades/Character/Skill/Common/Special.Special_C")))
            (bind _actor (CallFunction|SelectMinDistance _array "0, 0, 0"))
            (bind _asbase_enemy_bp_2 (Utilities|Casting|CastToBaseEnemy_BP _actor))
            (Default|SetCount _asbase_enemy_bp_2)
            (Actor|DestroyActor)))))))

(event EventTick
  (params (DeltaSeconds :type Float%20%28single-precision%29))
  (bind _returnvalue (Transformation|GetActorLocation))
  ;[1 1 1] DestroyAutomaticly
  (CallFunction|MoveForward DeltaSeconds)
  (if (Utilities|IsValid (Variables|Default|GetTarget))
    (CallFunction|AdjustRotation)
    (bind _output_get (Variables|Default|SetDistance (+ (Math|Vector|VectorLength (- _returnvalue (Variables|Default|GetLastPos))) (Variables|Default|GetDistance)) :!label _label))
    (Variables|Default|SetLastPos (Transformation|GetActorLocation))
    (if (>= _output_get (Variables|Default|GetMaxDistance))
      (bind _returnvalue_2 (Game|SpawnActorfromClass "/Game/Hades/Items/PickableItem_BP.PickableItem_BP_C" (Math|Transform|MakeTransform (Transformation|GetActorLocation) "0, 0, 0" "1,1,1") "Undefined" 0 0))
      (Transformation|SetMobility _returnvalue_2 "Movable")
      (Actor|DestroyActor))
    (else
      (bind (_outhit _returnvalue_3) (Collision|SphereTraceForObjects _returnvalue _returnvalue 5e+02 (Utilities|Array|MakeArray "ObjectTypeQuery3") false (Utilities|Array|MakeArray (Game|GetPlayerCharacter 0)) "None"))
      (if _returnvalue_3
        (Variables|Default|SetTarget (.hitactor _outhit))
        (else
          (goto _label))))))

(fn ConstructionScript
  (bind _output_get (Variables|Default|SetStartPos (Transformation|GetActorLocation)))
  (Variables|Default|SetLastPos _output_get))

(fn SetMaxDistance
  (params (MaxDistance :type Float%20%28single-precision%29))
  (Variables|Default|SetMaxDistance MaxDistance))

(fn SelectMinDistance
  (params (Array :type Array%20of%20Actor%20Object%20References) (Loc :type Vector))
  (LocalVariables|SetLength (Math|Vector|VectorLength (- (Transformation|GetActorLocation (Utilities|Array|Get(acopy) Array (LocalVariables|GetminIndex))) Loc)))
  (for (_array_element _array_index) Array
    (if (< (Math|Vector|VectorLength (- (Transformation|GetActorLocation _array_element) Loc)) (LocalVariables|GetLength))
      (LocalVariables|SetminIndex _array_index)
      (LocalVariables|SetLength (Math|Vector|VectorLength (- (Transformation|GetActorLocation _array_element) Loc)))))
  (return (Utilities|Array|Get(acopy) (Variables|Default|GetArray) (LocalVariables|GetminIndex))))

(fn AdjustRotation
  (bind _returnvalue (Transformation|GetActorForwardVector))
  (bind _returnvalue_2 (Transformation|GetActorLocation))
  (bind _returnvalue_3 (Transformation|GetActorRotation))
  (bind _target (Variables|Default|GetTarget))
  (bind (_x _y) (Math|Vector|BreakVector _returnvalue))
  (bind _returnvalue_4 (Transformation|GetActorLocation _target))
  (bind _returnvalue_5 (- _returnvalue_4 _returnvalue_2))
  (bind (_x_2 _y_2) (Math|Vector|BreakVector _returnvalue_5))
  (LocalVariables|SetVForward (Math|Vector|Normalize (Math|Vector|MakeVector _x _y 0.0)))
  (LocalVariables|SetVTarget (Math|Vector|Normalize (Math|Vector|MakeVector _x_2 _y_2 0.0)))
  (if (>= (.Z (Math|Vector|BreakVector (Math|Vector|CrossProduct (LocalVariables|GetVForward) (LocalVariables|GetVTarget)))) 0.0)
    (LocalVariables|SetLeft? true)
    (LocalVariables|SetDegrees (+ (Class|KismetMathLibrary|DegAcos (Math|Vector|DotProduct (LocalVariables|GetVForward) (LocalVariables|GetVTarget))) (.yaw (Transformation|GetActorRotation))))
    (else
      (LocalVariables|SetLeft? false)
      (LocalVariables|SetDegrees (- (.yaw (Transformation|GetActorRotation)) (Class|KismetMathLibrary|DegAcos (Math|Vector|DotProduct (LocalVariables|GetVForward) (LocalVariables|GetVTarget)))))))
  (Transformation|SetActorRotation (Math|Rotator|MakeRotator (.roll _returnvalue_3) (.pitch _returnvalue_3) (Math|Float|Lerp (.yaw _returnvalue_3) (LocalVariables|GetDegrees) 0.5))))

(fn MoveForward
  (params (DeltaTime :type Float%20%28single-precision%29))
  (Transformation|SetActorLocation (+ (Transformation|GetActorLocation) (* (* (Transformation|GetActorForwardVector) DeltaTime) (Variables|Default|GetSpeed))) true false))