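; Base skill component that deals area damage in front of its owning actor and exposes its Range.
; DoDamage sweeps a box trace for Pawn objects along the owner's forward vector, aligned to its rotation, with timed debug drawing.
; Hit actors are collected uniquely into an array, then each receives the component's Damage with the owner as damage causer.
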(fn DoDamage
  (bind _returnvalue (Components|GetOwner))
  (bind _array (Variables|Default|GetArray))
  (bind _returnvalue_2 (Transformation|GetActorLocation _returnvalue))
  (bind _outhits (Class|KismetSystemLibrary|BoxTraceMultiforObjects _returnvalue_2 (+ _returnvalue_2 (* (Transformation|GetActorForwardVector _returnvalue) (Math|Float|Truncate (Variables|Default|GetRange)))) (Variables|Default|GetHalfSize) (Transformation|GetActorRotation _returnvalue) (Utilities|Array|MakeArray "ObjectTypeQuery3") false 0 "ForDuration" true "(R=1.000000,G=0.000000,B=0.000000,A=1.000000)" "(R=0.000000,G=1.000000,B=0.000000,A=1.000000)" 2.0))
  (for _array_element _outhits
    (Utilities|Array|AddUnique _array (.hitactor _array_element)))
  (for _array_element_2 _array
    (Game|Damage|ApplyDamage _array_element_2 (Math|Conversions|ToFloat(Integer) (Variables|Default|GetDamage)) 0 (Components|GetOwner) "/Game/Hades/Character/Skill/Common/Normal.Normal_C")))

(fn ReturnRange
  (return (Variables|Default|GetRange)))