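; Base door Blueprint for Hades that sends the player to the next level when an actor overlaps it.
; On BeginPlay it sets a default door type in its DoorDescription and caches the GameManager_BP found in the level.
; On overlap it writes that door type to DoorOut on the Hades_Instance game instance, then calls NextLevel on the game manager.
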(event EventBeginPlay
  (Variables|/Game/Hades/Maps/Doors/DoorDescription.DoorDescription_C|SetType (Variables|Default|GetDoorDescription) "NewEnumerator4")
  (bind _returnvalue (Actor|GetActorOfClass "/Game/Hades/Maps/GameManager_BP.GameManager_BP_C"))
  (Variables|Default|SetGM _returnvalue))

(event Collision|EventActorBeginOverlap
  (params (OtherActor :type Actor%20Object%20Reference))
  (bind _ashades_instance (Utilities|Casting|CastToHades_Instance (Game|GetGameInstance)))
  (Variables|/Game/Hades/Hades_Instance.Hades_Instance_C|SetDoorOut _ashades_instance (Variables|/Game/Hades/Maps/Doors/DoorDescription.DoorDescription_C|GetType (Variables|Default|GetDoorDescription)))
  (Default|NextLevel (Variables|Default|GetGM)))

(fn ConstructionScript)