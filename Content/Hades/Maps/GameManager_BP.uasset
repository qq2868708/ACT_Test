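; Room manager for a Hades-style game with randomly linked maps, handling doors, enemy spawns and room completion.
; SearchDoors sorts doors by side; UpdateDoors uses the GameInstance's DoorOut to place the player at an opposite-side door and gather exit doors.
; Init spawns two enemy types at random navigable points; CheckEnd drops an item and enables exit collision once none remain.
; LoadLevel opens a random map from the opposite-side list for DoorOut.
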(event EventBeginPlay
  (Variables|Default|SetActor (Game|GetPlayerCharacter 0))
  (bind _ashades_instance (Utilities|Casting|CastToHades_Instance (Game|GetGameInstance)))
  (Variables|Default|SetGameInstance _ashades_instance))

(fn ConstructionScript)

(fn SearchDoors
  (bind _outactors (Actor|GetAllActorsOfClass "/Game/Hades/Maps/Doors/BaseDoor_BP.BaseDoor_BP_C"))
  (bind _output_get (Variables|Default|SetDoors_ALL _outactors))
  (for _array_element _output_get
    (switch Utilities|FlowControl|Switch|SwitchonDoor_Type (Variables|/Game/Hades/Maps/Doors/DoorDescription.DoorDescription_C|GetType (Actor|GetComponentbyClass _array_element "/Game/Hades/Maps/Doors/DoorDescription.DoorDescription_C"))
      (:NewEnumerator3
        (Utilities|Array|AddUnique (Variables|Default|GetDoors_L) _array_element))
      (:NewEnumerator1
        (Utilities|Array|AddUnique (Variables|Default|GetDoors_B) _array_element))
      (:NewEnumerator0
        (Utilities|Array|AddUnique (Variables|Default|GetDoors_T) _array_element))
      (:NewEnumerator2
        (Utilities|Array|AddUnique (Variables|Default|GetDoors_R) _array_element)))))

(fn SetDoors
  (params (Visable :type Boolean) (Array :type Array%20of%20Trigger%20Box%20Object%20References))
  (for _array_element Array
    (Collision|SetActorEnableCollision _array_element Visable)))

(fn UpdateDoors
  (switch Utilities|FlowControl|Switch|SwitchonDoor_Type (Variables|/Game/Hades/Hades_Instance.Hades_Instance_C|GetDoorOut (Variables|Default|GetGameInstance))
    (:NewEnumerator4
      (for _array_element (Variables|Default|GetDoors_ALL)
        (Utilities|Array|AddUnique (Variables|Default|GetDoorsOut) _array_element)))
    (:NewEnumerator3
      (bind (_doorin _door) (CallFunction|SelectDoors (Variables|Default|GetDoors_R)))
      (Transformation|SetActorLocation (Variables|Default|GetActor) _doorin false false)
      (Transformation|SetActorRelativeRotation (Variables|Default|GetActor) "0,-90.000000, 0")
      (for _array_element_2 (Variables|Default|GetDoors_ALL)
        (if (!= _array_element_2 _door)
          (Utilities|Array|AddUnique (Variables|Default|GetDoorsOut) _array_element_2))))
    (:NewEnumerator1
      (bind (_doorin_2 _door_2) (CallFunction|SelectDoors (Variables|Default|GetDoors_T)))
      (Transformation|SetActorLocation (Variables|Default|GetActor) _doorin_2 false false)
      (Transformation|SetActorRelativeRotation (Variables|Default|GetActor) "0,180.000000, 0")
      (for _array_element_3 (Variables|Default|GetDoors_ALL)
        (if (!= _array_element_3 _door_2)
          (Utilities|Array|AddUnique (Variables|Default|GetDoorsOut) _array_element_3))))
    (:NewEnumerator0
      (bind (_doorin_3 _door_3) (CallFunction|SelectDoors (Variables|Default|GetDoors_B)))
      (Transformation|SetActorLocation (Variables|Default|GetActor) _doorin_3 false false)
      (Transformation|SetActorRelativeRotation (Variables|Default|GetActor))
      (for _array_element_4 (Variables|Default|GetDoors_ALL)
        (if (!= _array_element_4 _door_3)
          (Utilities|Array|AddUnique (Variables|Default|GetDoorsOut) _array_element_4))))
    (:NewEnumerator2
      (bind (_doorin_4 _door_4) (CallFunction|SelectDoors (Variables|Default|GetDoors_L)))
      (Transformation|SetActorLocation (Variables|Default|GetActor) _doorin_4 false false)
      (Transformation|SetActorRelativeRotation (Variables|Default|GetActor) "0,90.000000, 0")
      (for _array_element_5 (Variables|Default|GetDoors_ALL)
        (if (!= _array_element_5 _door_4)
          (Utilities|Array|AddUnique (Variables|Default|GetDoorsOut) _array_element_5))))))

(fn SelectDoors
  (params (Array :type Array%20of%20Trigger%20Box%20Object%20References))
  (bind _returnvalue (Utilities|Array|Length Array))
  (bind _returnvalue_2 (Math|Random|RandomInteger _returnvalue))
  (bind _output (Utilities|Array|Get(acopy) Array _returnvalue_2))
  (return (+ (Transformation|GetActorLocation _output) (* (Transformation|GetActorForwardVector _output) 1e+02)) _output))

(fn ResetDoorOut
  (Variables|/Game/Hades/Hades_Instance.Hades_Instance_C|SetDoorOut (Variables|Default|GetGameInstance) "NewEnumerator4"))

(fn Init
  (bind _returnvalue (Math|Vector|VectorZero))
  (bind _randomlocation (AI|Navigation|GetRandomReachablePointinRadius _returnvalue 1e+05 0 0))
  (for _index (range 0 (Variables|Default|GetEnemyCount))
    (if (== (Math|Random|RandomInteger 2) 0)
      (bind _returnvalue_2 (Game|SpawnActorfromClass "/Game/Hades/AI/EnemyNew/近战兵/BaseEnemy_BP_Child1.BaseEnemy_BP_Child1_C" (Math|Transform|MakeTransform _randomlocation "0, 0, 0" "1,1,1") "Undefined" 0 0))
      (if (Utilities|IsValid _returnvalue_2)
        (Pawn|SpawnDefaultController _returnvalue_2)
        (Variables|/Script/Engine.Pawn|SetAIControllerClass _returnvalue_2 "/Game/Hades/AI/EnemyNew/近战兵/EnemyController_BP.EnemyController_BP_C"))
      (else
        (bind _returnvalue_3 (Game|SpawnActorfromClass "/Game/Hades/AI/EnemyNew/远程兵/BaseEnemy_BP_Child2.BaseEnemy_BP_Child2_C" (Math|Transform|MakeTransform _randomlocation "0, 0, 0" "1,1,1") "Undefined" 0 0))
        (if (Utilities|IsValid _returnvalue_3)
          (Pawn|SpawnDefaultController _returnvalue_3)
          (Variables|/Script/Engine.Pawn|SetAIControllerClass _returnvalue_3 "/Game/Hades/AI/EnemyNew/远程兵/EnemyController_SpecialAttack_BP.EnemyController_SpecialAttack_BP_C"))))))

(fn LoadLevel
  (bind _gameinstance (Variables|Default|GetGameInstance))
  (switch Utilities|FlowControl|Switch|SwitchonDoor_Type (Variables|/Game/Hades/Hades_Instance.Hades_Instance_C|GetDoorOut (Variables|Default|GetGameInstance))
    (:NewEnumerator3
      (bind _index (CallFunction|SelectLevel (Variables|/Game/Hades/Hades_Instance.Hades_Instance_C|GetR_Doors _gameinstance)))
      (Variables|Default|SetSelected true)
      (Game|OpenLevel(byName) (Utilities|String|StringToName (Utilities|String|Append "Map" (Utilities|String|ToString(Integer) _index)))))
    (:NewEnumerator1
      (bind _index_2 (CallFunction|SelectLevel (Variables|/Game/Hades/Hades_Instance.Hades_Instance_C|GetT_Doors _gameinstance)))
      (Variables|Default|SetSelected true)
      (Game|OpenLevel(byName) (Utilities|String|StringToName (Utilities|String|Append "Map" (Utilities|String|ToString(Integer) _index_2)))))
    (:NewEnumerator0
      (bind _index_3 (CallFunction|SelectLevel (Variables|/Game/Hades/Hades_Instance.Hades_Instance_C|GetB_Doors _gameinstance)))
      (Variables|Default|SetSelected true)
      (Game|OpenLevel(byName) (Utilities|String|StringToName (Utilities|String|Append "Map" (Utilities|String|ToString(Integer) _index_3)))))
    (:NewEnumerator2
      (bind _index_4 (CallFunction|SelectLevel (Variables|/Game/Hades/Hades_Instance.Hades_Instance_C|GetL_Doors _gameinstance)))
      (Variables|Default|SetSelected true)
      (Game|OpenLevel(byName) (Utilities|String|StringToName (Utilities|String|Append "Map" (Utilities|String|ToString(Integer) _index_4)))))))

(fn SelectLevel
  (params (Array :type Array%20of%20Integers))
  (return (Utilities|Array|Get(acopy) Array (Math|Random|RandomInteger (Utilities|Array|Length Array)))))

(fn CheckEnd
  (bind _returnvalue (Game|GetPlayerCharacter 0))
  (bind _outactors (Actor|GetAllActorsOfClass "/Game/Hades/AI/BaseAICharacter/BaseEnemy_BP.BaseEnemy_BP_C"))
  (if (<= (Utilities|Array|Length _outactors) 0)
    (Variables|Default|SetEnd true)
    (bind _returnvalue_2 (Game|SpawnActorfromClass "/Game/Hades/Items/Item_BP.Item_BP_C" (Math|Transform|MakeTransform (+ (Transformation|GetActorLocation _returnvalue) (* (Transformation|GetActorForwardVector _returnvalue) 1e+02)) "0, 0, 0" "1,1,1") "Undefined" 0 0))
    (Transformation|SetMobility _returnvalue_2 "Movable")
    (CallFunction|SetDoors true (Variables|Default|GetDoorsOut))
    (CallFunction|ResetDoorOut)))