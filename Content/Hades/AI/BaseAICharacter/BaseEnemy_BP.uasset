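; Base enemy AI character that tracks health, links itself to its health bar widget, and reacts to damage.
; Each hit reduces health and turns the enemy toward the damage causer, then plays a hurt montage if it survives; the knockback impulse is zeroed out.
; Special-type hits increment a count that sets how many pickups scatter on death.
; Death detaches the controller, disables collision, then destroys the actor after a delay and notifies GM.
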(event Game|Damage|EventAnyDamage
  (params (Damage :type Float%20%28single-precision%29) (DamageType :type Damage%20Type%20Object%20Reference) (InstigatedBy :type Controller%20Object%20Reference) (DamageCauser :type Actor%20Object%20Reference))
  (bind _returnvalue (Transformation|GetActorLocation))
  ;[1 1 1] HurtAndDead
  (bind _asbase_damage_type (Utilities|Casting|CastToBaseDamageType DamageType)
    (:then
      (switch Utilities|FlowControl|Switch|SwitchonDamageType (Variables|/Game/Hades/Character/Skill/Common/BaseDamageType.BaseDamageType_C|GetDamageType _asbase_damage_type)
        (:NewEnumerator0
          _)
        (:NewEnumerator1
          (Variables|Default|SetCount (+ (Variables|Default|GetCount) 1)))))
    (:CastFailed
      _))
  (if (Utilities|IsValid DamageCauser)
    (Variables|Default|SetCauser (Transformation|GetActorLocation DamageCauser)))
  (if (not (Variables|Default|GetDead))
    (CallFunction|UpdateHp Damage)
    (Transformation|SetActorRotation (Math|Rotator|FindLookatRotation _returnvalue (+ _returnvalue (Math|Vector|Normalize (- (Variables|Default|GetCauser) (Transformation|GetActorLocation))))))
    (if (Variables|Default|GetDead)
      (Variables|Default|SetBeAttacked true)
      (Variables|Default|SetDead true)
      (Variables|Default|SetCanAttack false)
      (Class|Pawn|DetachfromControllerPendingDestroy)
      (Collision|SetCollisionEnabled (Variables|Collision|GetCapsuleComponent) "NoCollision")
      (for _index (range 1 (Variables|Default|GetCount))
        (bind _newparam (CallFunction|RandomVector))
        (bind _returnvalue_2 (Game|SpawnActorfromClass "/Game/Hades/Items/PickableItem_BP.PickableItem_BP_C" (Math|Transform|MakeTransform (+ (Transformation|GetActorLocation) (* _newparam (Math|Random|RandomInteger 200))) "0, 0, 0" "1,1,1") "Undefined" 0 0))
        (Transformation|SetMobility _returnvalue_2 "Movable"))
      (Rendering|SetVisibility (Variables|Default|GetHealthUI) false false)
      (Utilities|FlowControl|Delay 3.0)
      (Actor|DestroyActor)
      (Default|EnemyDead (Variables|Default|GetGM))
      (else
        (Physics|AddImpulse (Variables|Character|GetCharacterMovement) (* (* (Transformation|GetActorForwardVector) 0.0) -30000) false)
        (Variables|Default|SetBeAttacked true)
        (bind _returnvalue_3 (Animation|PlayAnimMontage "/Game/Hades/Hurt_Heavy_Inplace.Hurt_Heavy_Inplace" 1.0 "None"))
        (Utilities|FlowControl|Delay _returnvalue_3)
        (Variables|Default|SetBeAttacked false)))))

(event EventBeginPlay
  ;[1 1 1] Init
  (Variables|Default|SetCurrentHealth 100)
  (Variables|Default|SetMaxHealth 100)
  (bind _asenemy_health_bar_bp (Utilities|Casting|CastToEnemyHealthBar_BP (UserInterface|GetWidget (Variables|Default|GetHealthUI))))
  (Variables|/Game/Hades/UI/EnemyHealthBar_BP.EnemyHealthBar_BP_C|SetAIActor _asenemy_health_bar_bp self))

(fn ConstructionScript)

(fn SetCauserSource
  (params (Pos :type Vector))
  (Variables|Default|SetCauser Pos))

(fn UpdateHp
  (params (Damage :type Float%20%28single-precision%29))
  (bind _output_get (Variables|Default|SetCurrentHealth (- (Variables|Default|GetCurrentHealth) (Math|Float|Truncate Damage))))
  (if (<= _output_get 0)
    (Variables|Default|SetCurrentHealth 0)
    (Variables|Default|SetDead (<= _output_get 0))))

(fn RandomVector
  (return (Math|Vector|Normalize (Math|Vector|MakeVector (Math|Random|RandomFloat) (Math|Random|RandomFloat) 0.0))))