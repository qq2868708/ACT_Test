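; Enemy magic projectile that damages living Hades_BP characters on impact and destroys itself.
; On a hit with anything but its owner, a sphere trace gathers unique nearby pawns, then sets the damage source position and applies damage to each living Hades_BP.
; Tick destroys it once a running distance total reaches the settable maximum; LastPos is never updated, so each tick adds the full offset from spawn.
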(event EventTick
  (params (DeltaSeconds :type Float%20%28single-precision%29))
  ;[1 1 1] DestroyAutomaticly
  (bind _output_get (Variables|Default|SetDistance (+ (Math|Vector|VectorLength (- (Transformation|GetActorLocation) (Variables|Default|GetLastPos))) (Variables|Default|GetDistance))))
  (if (>= _output_get (Variables|Default|GetMaxDistance))
    (Actor|DestroyActor)))

(event Collision|EventHit
  (params (MyComp :type Primitive%20Component%20Object%20Reference) (Other :type Actor%20Object%20Reference) (OtherComp :type Primitive%20Component%20Object%20Reference) (bSelfMoved :type Boolean) (HitLocation :type Vector :default "0, 0, 0") (HitNormal :type Vector :default "0, 0, 0") (NormalImpulse :type Vector :default "0, 0, 0") (Hit :type Hit%20Result%20Structure%20%28by%20ref%29))
  (bind _returnvalue (Transformation|GetActorLocation))
  (bind _array (Variables|Default|GetArray))
  ;[1 1 1] Comment
  (if (not (== Other (Variables|Default|GetOwnerActor)))
    (Variables|Default|SetSelfPos _returnvalue)
    (bind _outhits (Collision|MultiSphereTraceForObjects _returnvalue _returnvalue 1e+02 (Utilities|Array|MakeArray "ObjectTypeQuery3") false 0 "None" true "(R=1.000000,G=0.000000,B=0.000000,A=1.000000)" "(R=0.000000,G=1.000000,B=0.000000,A=1.000000)" 2.0))
    (if (<= (Utilities|Array|Length _outhits) 0)
      (Actor|DestroyActor)
      (else
        (for _array_element _outhits
          (Utilities|Array|AddUnique _array (.hitactor _array_element)))
        (if (<= (Utilities|Array|Length _array) 0)
          (Actor|DestroyActor)
          (else
            (for _array_element_2 (Variables|Default|GetArray)
              (bind _ashades_bp (Utilities|Casting|CastToHades_BP _array_element_2))
              (if (not (Variables|/Game/Hades/Character/Hades_BP.Hades_BP_C|GetDead _ashades_bp))
                (Default|SetCauserSource _ashades_bp (Variables|Default|GetSelfPos))
                (Game|Damage|ApplyDamage _array_element_2 2.0 0 0)))
            (Actor|DestroyActor)))))))

(fn ConstructionScript
  (bind _output_get (Variables|Default|SetStartPos (Transformation|GetActorLocation)))
  (Variables|Default|SetLastPos _output_get))

(fn SetMaxDistance
  (params (MaxDistance :type Float%20%28single-precision%29))
  (Variables|Default|SetMaxDistance MaxDistance))