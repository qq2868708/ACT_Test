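; Enemy Blueprint that reacts to taking damage with a hurt animation and knockback.
; On AnyDamage it turns on the horizontal plane to face the stored causer position, plays a heavy in-place hurt montage, and applies a backward impulse scaled by damage.
; The position comes from a valid damage causer, or otherwise keeps its previous value, which SetCauserSource can also set.
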(event Game|Damage|EventAnyDamage
  (params (Damage :type Float%20%28single-precision%29) (DamageType :type Damage%20Type%20Object%20Reference) (InstigatedBy :type Controller%20Object%20Reference) (DamageCauser :type Actor%20Object%20Reference))
  (bind _returnvalue (Transformation|GetActorLocation))
  ;[1 1 1] Hurt
  (if (Utilities|IsValid DamageCauser)
    (Variables|Default|SetCauser (Transformation|GetActorLocation DamageCauser)))
  (Transformation|SetActorRotation (Math|Rotator|FindLookatRotation _returnvalue (+ _returnvalue (Math|Vector|Normalize (Math|Vector|MakeVector (.X (Math|Vector|BreakVector (- (Variables|Default|GetCauser) (Transformation|GetActorLocation)))) (.Y (Math|Vector|BreakVector (- (Variables|Default|GetCauser) (Transformation|GetActorLocation)))) 0.0)))))
  (Animation|PlayAnimMontage "/Game/Hades/Hurt_Heavy_Inplace.Hurt_Heavy_Inplace" 1.0 "None")
  (Physics|AddImpulse (Variables|Character|GetCharacterMovement) (* (* (Transformation|GetActorForwardVector) Damage) -30000) false))

(fn ConstructionScript)

(fn SetCauserSource
  (params (Pos :type Vector))
  (Variables|Default|SetCauser Pos))