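; BP_SkillComponent is a skill component that deals melee-range knock-down damage in front of its owning actor.
; DoDamage runs a short box trace along the owner's forward vector against Pawn objects, with timed debug drawing.
; Hit actors are gathered uniquely into an array, then each receives damage using the knock-down damage type, with the owner as causer.
; The OnCastImp event is an empty stub, and nothing in the graphs calls DoDamage.
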(event EventOnCastImp)

(fn DoDamage
  (bind _returnvalue (Components|GetOwner))
  (bind _returnvalue_2 (Transformation|GetActorLocation _returnvalue))
  (bind _outhits (Class|KismetSystemLibrary|BoxTraceMultiforObjects _returnvalue_2 (+ _returnvalue_2 (* (Transformation|GetActorForwardVector _returnvalue) 1e+02)) "0,50.000000,50.000000" (Transformation|GetActorRotation _returnvalue) (Utilities|Array|MakeArray "ObjectTypeQuery3") false 0 "ForDuration" true))
  (for _array_element _outhits
    (Utilities|Array|AddUnique (LocalVariables|GetActors) (.hitactor _array_element)))
  (for _array_element_2 (LocalVariables|GetActors)
    (Game|Damage|ApplyDamage _array_element_2 5.0 0 (Components|GetOwner) "/Game/BP_DamageType_Base_KnockDown.BP_DamageType_Base_KnockDown_C")))